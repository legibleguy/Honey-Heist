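; BP_MeshGridTool is a construction-time tool that lays out a chosen mesh in an X by Y grid.
; The construction script assigns the mesh to an InstancedStaticMesh component and adds one instance per cell in a nested loop.
; Cell spacing comes from the mesh's bounding box size, and a shared Offset shifts every instance by the same amount.
; It has no active runtime logic.
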(fn `UserConstructionScript`
  (locals (CurrX :type Integer) (CurrY :type Integer))
  (bind (_returnvalue_origin _returnvalue_boxextent) (`KismetMathLibrary.BreakBoxSphereBounds` (`StaticMesh.GetBounds` (`self.Mesh`))))
  (`StaticMeshComponent.SetStaticMesh` (`self.InstancedStaticMesh`) (`self.Mesh`))
  (set `self.Extent` _returnvalue_boxextent)
  (for _index (range (`self.X`))
    (set `local.CurrX` _index)
    (for _index_2 (range (`self.Y`))
      (set `local.CurrY` _index_2)
      (`InstancedStaticMeshComponent.AddInstance` (`self.InstancedStaticMesh`) (`KismetMathLibrary.MakeTransform` (+ (* (* (`self.Extent`) 2) (`KismetMathLibrary.MakeVector` (`KismetMathLibrary.Conv_IntToDouble` (`local.CurrX`)) (`KismetMathLibrary.Conv_IntToDouble` (`local.CurrY`)))) (`self.Offset`)))))))