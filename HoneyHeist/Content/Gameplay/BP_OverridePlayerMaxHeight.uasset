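; Trigger actor that changes the player bee's flight height limit and ground level when the bee enters it.
; It sets BP_BeePawn's MaxHeight and GroundLevel to its own values, or to the HoneyHeist_Management table height and zero ground when ResetHeightToDefault is set.
; Tick also applies this once while a bee overlaps, through a DoOnce that re-arms on player exit.
; Leaving the actor does not restore previous values.
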(event `self.ReceiveActorBeginOverlap`
  (params (OtherActor :type "Actor Object Reference"))
  (if (== OtherActor (`GameplayStatics.GetPlayerPawn` 0))
    (bind _returnvalue (`|GetDataTableRow` "/Game/HoneyHeist_Management.HoneyHeist_Management" "NewRow" :!label _label)
      (:`then`
        (bind _asbp_bee_pawn (cast `/Game/Gameplay/BeeAndBear/BP_BeePawn` (`GameplayStatics.GetPlayerPawn` 0)))
        (set `/Game/Gameplay/BeeAndBear/BP_BeePawn.MaxHeight` (`KismetMathLibrary.SelectFloat` (`.MaxFlightHeight_24_0C7D52004A97EF7E23DD5EBC08527137` (break `/Game/Data/GameplayParameters` _returnvalue)) (`self.NewMaxHeight`) (`self.ResetHeightToDefault`)) _asbp_bee_pawn)
        (set `/Game/Gameplay/BeeAndBear/BP_BeePawn.GroundLevel` (`KismetMathLibrary.SelectFloat` 0.0 (`self.GroundLvl`) (`self.ResetHeightToDefault`)) _asbp_bee_pawn)))))

(event `self.ReceiveTick`
  (params (DeltaSeconds :type "Float (single-precision)"))
  (if (> (`KismetArrayLibrary.Array_Length` (`self.GetOverlappingActors` "/Game/Gameplay/BeeAndBear/BP_BeePawn.BP_BeePawn_C")) 0)
    (`/Engine/EditorBlueprintResources/StandardMacros.DoOnce` false :!label _label_2
      (:`Completed`
        (goto _label)))))

(event `self.ReceiveActorEndOverlap`
  (params (OtherActor :type "Actor Object Reference"))
  (if (== OtherActor (`GameplayStatics.GetPlayerPawn` 0))
    (goto _label_2 :!via `Reset`)))

(fn `UserConstructionScript`)