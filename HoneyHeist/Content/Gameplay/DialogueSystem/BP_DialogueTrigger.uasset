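; BP_DialogueTrigger is an overlap trigger actor that starts its assigned dialogue when the player pawn enters it.
; It stores the pawn's transform and teleports the pawn back to it every Tick, freezing the player in place.
; It relays dialogue start and progress through its own dispatchers.
; Only with AutoDestroy does it relay completion and destroy itself, ending the lock, as Active is never cleared.
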(event `self.ReceiveActorBeginOverlap`
  (params (OtherActor :type "Actor Object Reference"))
  (if (== OtherActor (`GameplayStatics.GetPlayerPawn` 0))
    (set `self.Active` true)
    (set `self.Tr` (`self.GetTransform` (`GameplayStatics.GetPlayerPawn` 0)))
    (bind _outdialogueobject (`/Game/Gameplay/DialogueSystem/DialogueSystem.StartDialogue` (`GameplayStatics.GetPlayerController` 0) (`self.DialogueToPlay`)))
    (bind _output_get (set `self.DialogueObj` _outdialogueobject))
    (`self.DialogueStarted`)
    (add `/Game/Gameplay/DialogueSystem/Dialogue.DialogueFinished` _output_get (delegate `OnDIalogueFInished`))
    (add `/Game/Gameplay/DialogueSystem/Dialogue.OnDialogueProceed` (`self.DialogueObj`) (delegate `OnDialogueProceed`))))

(event `self.ReceiveTick`
  (params (DeltaSeconds :type "Float (single-precision)"))
  (if (`self.Active`)
    (`self.K2_SetActorTransform` (`GameplayStatics.GetPlayerPawn` 0) (`self.Tr`) false true)))

(event `OnDialogueProceed`
  (params (CurrIndex :type Integer))
  (`self.DialogueProceed` CurrIndex))

(event `OnDIalogueFInished`
  (if (`self.AutoDestroy`)
    (`self.DialogueFinished`)
    (`self.K2_DestroyActor`)))

(fn `UserConstructionScript`)