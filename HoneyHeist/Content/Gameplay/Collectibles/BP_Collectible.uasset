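; BP_Collectible is a pickup actor that the player collects by touching it.
; On overlap with player 0's pawn, it sends that pawn an OnItemCollected message, plays a pickup sound and destroys itself.
; The construction script sets the collision sphere's size from a Radius variable.
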(event `self.ReceiveActorBeginOverlap`
  (params (OtherActor :type "Actor Object Reference"))
  (if (== OtherActor (`GameplayStatics.GetPlayerPawn` 0))
    (message `/Game/Gameplay/BeeGame_IF.OnItemCollected` OtherActor)
    (`GameplayStatics.PlaySoundAtLocation` (`self.PickUpSound`) (0.0 0.0 0.0) (struct) 1.0 1.0 0.0 null null self)
    (`self.K2_DestroyActor`)))

(fn `UserConstructionScript`
  (`SphereComponent.SetSphereRadius` (`self.Sphere`) (`self.Radius`) true))