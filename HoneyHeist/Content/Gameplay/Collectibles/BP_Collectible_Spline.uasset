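; Spline-based placer that lays out a row of collectibles along a path.
; The construction script derives the count from the spline length, the collectible class's default radius and a spacing value.
; It adds a child actor component of that class for each slot, spread evenly from start to end with constant-velocity sampling.
; The event graph has no active logic.
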(fn `UserConstructionScript`
  (locals (TotalCollectibles :type Integer :default 0))
  (bind _output_get (set `local.TotalCollectibles` (`KismetMathLibrary.FTrunc` (/ (`SplineComponent.GetSplineLength` (`self.Spline`)) (+ (* (`.Radius` (defaults `Object` (`self.CollectibleClass`))) 2.0) (`self.Spacing`))))))
  (for _index (range _output_get)
    (bind _returnvalue (`AddComponent|NODE_AddChildActorComponent-0` :`RelativeTransform` (`SplineComponent.GetTransformAtTime` (`self.Spline`) (/ (`KismetMathLibrary.Conv_IntToDouble` _index) (`KismetMathLibrary.Conv_IntToDouble` (- (`local.TotalCollectibles`) 1))) "Local" true false)))
    (`ChildActorComponent.SetChildActorClass` _returnvalue (`self.CollectibleClass`))))