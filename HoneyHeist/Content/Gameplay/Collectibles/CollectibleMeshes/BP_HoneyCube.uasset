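; BP_HoneyCube is a honey cube collectible that supplies navigation points around itself.
; On BeginPlay it runs the Patrol_FindTarget EQS query with itself as querier and caches all matching locations in PointsAround.
; GetPointsAroundObject exposes that cache, and a DebugNavigation flag draws the points.
; The character-state, movement, UI and remaining-time getters are stubs returning empty, false or zero values.
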(event `self.ReceiveBeginPlay`
  (`parent.ReceiveBeginPlay`)
  (bind _returnvalue (`EnvQueryManager.RunEQSQuery` "/Game/Gameplay/AI/Patrol_FindTarget.Patrol_FindTarget" self "AllMatching"))
  (add `EnvQueryInstanceBlueprintWrapper.OnQueryFinishedEvent` _returnvalue (delegate `QueryDone`)))

(event `QueryDone`
  (params (QueryInstance :type "EnvQueryInstanceBlueprintWrapper Object Reference") (QueryStatus :type "EEnvQueryStatus Enum" :default "Processing"))
  (bind _resultlocations (`EnvQueryInstanceBlueprintWrapper.GetQueryResultsAsLocations` QueryInstance))
  (bind _output_get (set `self.PointsAround` _resultlocations))
  (if (`self.DebugNavigation`)
    (for _array_element _output_get
      (`KismetSystemLibrary.DrawDebugPoint` _array_element 20.0 (struct :`G` 0.224473 :`B` 1.0 :`A` 1.0) 8.0))))

(fn `GetCharacterMovementInfo`
  (returns (MovementInput :type "Vector Structure"))
  (return (0.0 0.0 0.0)))

(fn `GetInGameUI`
  (returns (OutUI :type "UserWidget Object Reference"))
  (return null))

(fn `GetPointsAroundObject`
  (returns (OutPoints :type "Array of Vector Structure"))
  (return (`self.PointsAround`)))

(fn `IsCharacterAlive`
  (returns (IsAlive :type Boolean))
  (return false))

(fn `IsCharacterAwake`
  (returns (IsAwake :type Boolean))
  (return false))

(fn `RequestRemainingTime`
  (returns (OutTime :type "Float (double-precision)"))
  (return 0.0))

(fn `UserConstructionScript`
  (`parent.UserConstructionScript`))