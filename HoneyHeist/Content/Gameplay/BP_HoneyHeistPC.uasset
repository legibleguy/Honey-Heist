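; BP_HoneyHeistPC is the Honey Heist player controller, owning the in-game HUD and the pause menu.
; OnGameModeReady creates the InGame_UMG widget and sets GMReady, and an event toggles that widget's visibility.
; The Pause input flip-flops between opening and removing PauseMenu, switching game pause, cursor and UI visibility, restoring UI only if GMReady.
; GetInGameUI exposes the HUD, while the other query and boost functions are empty or default-value stubs.
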(event `/Game/Gameplay/BeeGame_IF.OnGameModeReady`
  (params (ExitLocation :type "Vector Structure"))
  (bind _returnvalue (`|CreateWidget` "/Game/UI/GameHUD/InGame_UMG.InGame_UMG_C" self))
  (bind _output_get (set `self.InGameUI` _returnvalue))
  (`UserWidget.AddToViewport` _output_get 0)
  (set `self.GM_Ready` true))

(event `self.ReceiveBeginPlay`)

(event `/Game/Gameplay/BeeGame_IF.SetGameUI_Visible`
  (params (Visible :type Boolean))
  (bind _ingameui (`self.InGameUI`)
    (:`then`
      (`Widget.SetVisibility` _ingameui (select `bool` Visible :`false` "Hidden" :`true` "Visible" :!type "ESlateVisibility Enum")))
    (:`else`)))

(event `InputAction|Pause` :paused true
  (params (Key :type "Key Structure"))
  (:`Pressed`
    (`/Engine/EditorBlueprintResources/StandardMacros.FlipFlop`
      (:`A`
        (bind _returnvalue (`|CreateWidget` "/Game/UI/GameHUD/PauseMenu.PauseMenu_C" self))
        (bind _output_get (set `self.PauseMenu` _returnvalue))
        (`UserWidget.AddToViewport` _output_get 0)
        (`/Game/Gameplay/HH_FunctionsLib.SetUI_Visibility` false)
        (`GameplayStatics.SetGamePaused` true)
        (set `self.bShowMouseCursor` true))
      (:`B`
        (`Widget.RemoveFromParent` (`self.PauseMenu`))
        (`GameplayStatics.SetGamePaused` false)
        (set `self.bShowMouseCursor` false)
        (if (`self.GM_Ready`)
          (`/Game/Gameplay/HH_FunctionsLib.SetUI_Visibility` true))))))

(fn `GetBoostLevel`
  (returns (BoostPercent :type "Float (double-precision)"))
  (return 0.0))

(fn `GetCharacterMovementInfo`
  (returns (MovementInput :type "Vector Structure"))
  (return (0.0 0.0 0.0)))

(fn `GetInGameUI`
  (returns (OutUI :type "UserWidget Object Reference"))
  (return (`self.InGameUI`)))

(fn `GetPointsAroundObject`
  (returns (OutPoints :type "Array of Vector Structure"))
  (return))

(fn `IsCharacterAlive`
  (returns (IsAlive :type Boolean))
  (return false))

(fn `IsCharacterAwake`
  (returns (IsAwake :type Boolean))
  (return false))

(fn `RequestRemainingTime`
  (returns (OutTime :type "Float (double-precision)"))
  (return 0.0))

(fn `SetPlayerBoosted`
  (params (Boosted :type Boolean))
  (return))

(fn `UserConstructionScript`)