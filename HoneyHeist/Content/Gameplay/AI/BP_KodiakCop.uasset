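; BP_KodiakCop is an AI cop that walks to the exit location supplied when the game mode is ready.
; Its move macro sets walk speed to navmesh path length divided by remaining time, timing arrival to the countdown.
; While it is nearly stationary, Tick runs a looping timer that checks its box for actors of the player pawn's class.
; An overlap triggers an attack, stops the timer and resumes the move.
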(event `self.ReceiveTick`
  (params (DeltaSeconds :type "Float (single-precision)"))
  (`parent.ReceiveTick` DeltaSeconds)
  (if (== (`self.GetVelocity`) (0.0 0.0 0.0) :`ErrorTolerance` 10.0)
    (if (not (`KismetSystemLibrary.K2_IsValidTimerHandle` (`self.PlayerCheckTimer`)))
      (bind _returnvalue (`KismetSystemLibrary.K2_SetTimerDelegate` (delegate `CheckIfCharacterIsObstacle`) 0.1 true))
      (set `self.PlayerCheckTimer` _returnvalue))
    (elif (`KismetSystemLibrary.K2_IsValidTimerHandle` (`self.PlayerCheckTimer`))
      (`KismetSystemLibrary.K2_ClearAndInvalidateTimerHandle` (`self.PlayerCheckTimer`)))))

(event `CheckIfCharacterIsObstacle`
  (if (> (`KismetArrayLibrary.Array_Length` (`PrimitiveComponent.GetOverlappingActors` (`self.Box`) (`GameplayStatics.GetObjectClass` (`GameplayStatics.GetPlayerPawn` 0)))) 0)
    (`self.AttackPlayer`)
    (`KismetSystemLibrary.K2_ClearAndInvalidateTimerHandle` (`self.PlayerCheckTimer`))
    (`self.MoveToFinishPoint`)))

(event `/Game/Gameplay/BeeGame_IF.OnGameModeReady`
  (params (ExitLocation :type "Vector Structure"))
  (set `self.FinishPoint` ExitLocation)
  (`self.MoveToFinishPoint`))

(fn `UserConstructionScript`
  (`parent.UserConstructionScript`))