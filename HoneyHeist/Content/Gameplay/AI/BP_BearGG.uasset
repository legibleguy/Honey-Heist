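; BP_BearGG is a bear AI Blueprint that patrols and chases the player.
; After calling its parent BeginPlay, it waits briefly and then calls StartPatrol.
; An AIPerception update for player pawn 0 calls ChasePlayer without checking whether the player was sensed or lost.
; StartPatrol and ChasePlayer are defined outside these graphs, and nothing here returns it to patrol.
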(event `self.ReceiveBeginPlay`
  (`parent.ReceiveBeginPlay`)
  (`KismetSystemLibrary.Delay` 0.2)
  (`self.StartPatrol`))

(event `self.AIPerception.OnTargetPerceptionUpdated`
  (params (Actor :type "Actor Object Reference") (Stimulus :type "AIStimulus Structure"))
  (if (== Actor (`GameplayStatics.GetPlayerPawn` 0))
    (`self.ChasePlayer`)))

(fn `UserConstructionScript`
  (`parent.UserConstructionScript`))