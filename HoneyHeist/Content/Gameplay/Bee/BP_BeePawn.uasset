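; BP_BeePawn is the player-controlled bee pawn, flying on a FloatingPawnMovement component.
; Axis inputs move it along control-rotation forward and right and actor up, and drive controller look.
; Keys 1 and 2 switch between follow-camera yaw and follow-velocity rotation, which Tick smooths toward the travel direction with RInterpTo.
; View-mode functions cycle third-person, first-person and top-down, toggling the third-person camera and setting the rotation mode.
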(event `self.ReceiveBeginPlay`
  (`self.UpdateRotationMode` "NewEnumerator1"))

(event `self.ReceiveTick`
  (params (DeltaSeconds :type "Float (single-precision)"))
  (bind (_returnvalue_roll _returnvalue_pitch _returnvalue_yaw) (`KismetMathLibrary.BreakRotator` (`KismetMathLibrary.MakeRotFromX` (`self.GetVelocity`))))
  (`|ExecutionSequence`
    (:`then_1`
      (switch `/Game/Gameplay/Bee/RotationMode` (`self.RotationMode`)
        (:`NewEnumerator1`
          (if (> (`KismetMathLibrary.VSize` (`self.GetVelocity`)) 0.0)
            (`self.K2_SetActorRotation` (`KismetMathLibrary.RInterpTo` (`self.K2_GetActorRotation`) (`KismetMathLibrary.MakeRotator` 0.0 0.0 _returnvalue_yaw) DeltaSeconds 5.0))))))))

(event `InputAxis|MoveFB`
  (params (AxisValue :type "Float (single-precision)"))
  (bind (_returnvalue_roll _returnvalue_pitch _returnvalue_yaw) (`KismetMathLibrary.BreakRotator` (`self.GetControlRotation`)))
  (`PawnMovementComponent.AddInputVector` (`self.FloatingPawnMovement`) (* (`KismetMathLibrary.GetForwardVector` (`KismetMathLibrary.MakeRotator` 0.0 _returnvalue_pitch _returnvalue_yaw)) AxisValue) false))

(event `Key|One`
  (params (Key :type "Key Structure"))
  (:`Pressed`
    (switch `/Game/Gameplay/Bee/CameraMode` (`self.CurrentViewMode`)
      (:`NewEnumerator0`
        _)
      (:`NewEnumerator3`
        _))
    (`self.UpdateRotationMode` "NewEnumerator0")))

(event `InputAxis|MoveRL`
  (params (AxisValue :type "Float (single-precision)"))
  (bind (_returnvalue_roll _returnvalue_pitch _returnvalue_yaw) (`KismetMathLibrary.BreakRotator` (`self.GetControlRotation`)))
  (`PawnMovementComponent.AddInputVector` (`self.FloatingPawnMovement`) (* (`KismetMathLibrary.GetRightVector` (`KismetMathLibrary.MakeRotator` 0.0 _returnvalue_pitch _returnvalue_yaw)) AxisValue) false))

(event `Key|Two`
  (params (Key :type "Key Structure"))
  (:`Pressed`
    (switch `/Game/Gameplay/Bee/CameraMode` (`self.CurrentViewMode`)
      (:`NewEnumerator0`
        (`self.UpdateRotationMode` "NewEnumerator1")))))

(event `InputAxis|LookRL`
  (params (AxisValue :type "Float (single-precision)"))
  (`self.AddControllerYawInput` AxisValue))

(event `InputAxis|LookUD`
  (params (AxisValue :type "Float (single-precision)"))
  (`self.AddControllerPitchInput` AxisValue))

(event `InputAxis|MoveUD`
  (params (AxisValue :type "Float (single-precision)"))
  (`PawnMovementComponent.AddInputVector` (`self.FloatingPawnMovement`) (* (`self.GetActorUpVector`) AxisValue) false))

(fn `ToggleView`
  (if (>= (+ (`KismetMathLibrary.Conv_ByteToInt` (`self.CurrentViewMode`)) 1) (enumcount `/Game/Gameplay/Bee/CameraMode`))
    (`self.UpdateVIewMode` "NewEnumerator0")
    (else
      (`self.UpdateVIewMode` (cast `/Game/Gameplay/Bee/CameraMode` (`KismetMathLibrary.Conv_IntToByte` (+ (`KismetMathLibrary.Conv_ByteToInt` (`self.CurrentViewMode`)) 1)))))))

(fn `UpdateRotationMode`
  (params (RotationMode :type "/Game/Gameplay/Bee/RotationMode Enum" :default "NewEnumerator0"))
  (bind _output_get (set `self.RotationMode` RotationMode))
  (`KismetSystemLibrary.PrintString` (`KismetStringLibrary.Concat_StrStr` "New Rotation Mode: " (`|GetEnumeratorNameAsString` _output_get)))
  (switch `/Game/Gameplay/Bee/RotationMode` (`self.RotationMode`)
    (:`NewEnumerator0`
      (set `self.bUseControllerRotationYaw` true))
    (:`NewEnumerator1`
      (switch `/Game/Gameplay/Bee/CameraMode` (`self.CurrentViewMode`)
        (:`NewEnumerator0`
          (set `self.bUseControllerRotationYaw` false)
          (`|ExecutionSequence`
            (:`then_0`
              (set `SpringArmComponent.bUsePawnControlRotation` true (`self.SA_TP`))
              (set `SpringArmComponent.bInheritYaw` true (`self.SA_TP`))
              (set `SpringArmComponent.bInheritPitch` true (`self.SA_TP`)))))
        (:`NewEnumerator3`
          (set `self.bUseControllerRotationYaw` false))))))

(fn `UpdateVIewMode`
  (params (NewMode :type "/Game/Gameplay/Bee/CameraMode Enum" :default "NewEnumerator0"))
  (bind _output_get (set `self.CurrentViewMode` NewMode))
  (`KismetSystemLibrary.PrintString` (`KismetStringLibrary.Concat_StrStr` "View mode updated: " (`|GetEnumeratorNameAsString` _output_get)))
  (switch `/Game/Gameplay/Bee/CameraMode` _output_get
    (:`NewEnumerator0`
      (`ActorComponent.SetActive` (`self.Camera_TP`) true false)
      (`self.UpdateRotationMode` "NewEnumerator1"))
    (:`NewEnumerator1`
      (`ActorComponent.SetActive` (`self.Camera_TP`) false false)
      (`self.UpdateRotationMode` "NewEnumerator0"))
    (:`NewEnumerator3`
      (`ActorComponent.SetActive` (`self.Camera_TP`) false false)
      (`self.UpdateRotationMode` "NewEnumerator1"))))

(fn `UserConstructionScript`)