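; Player bee pawn for the Honey Heist game that flies freely and counts collected honey cubes, printing the total each tick.
; Camera-relative input is interpolated each tick into FloatingPawnMovement, with climbing damped near max height.
; Rotation modes either follow velocity while idle or timeline-snap to the camera when moving, alongside switchable third-person, first-person and top-down view modes.
; Speed, acceleration, scale and height limit come from the HoneyHeist_Management data table.
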(event `self.ReceiveBeginPlay`
  (`self.UpdateRotationMode` "NewEnumerator1")
  (`self.UpdateFromManagementTable`))

(event `/Game/Gameplay/BeeGame_IF.OnItemCollected`
  (`/Engine/EditorBlueprintResources/StandardMacros.IncrementInt` (`self.HoneyCubeCount`)))

(event `self.ReceiveTick`
  (params (DeltaSeconds :type "Float (single-precision)"))
  (bind (_returnvalue_roll _returnvalue_pitch _returnvalue_yaw) (`KismetMathLibrary.BreakRotator` (`KismetMathLibrary.MakeRotFromX` (`self.GetVelocity`))))
  (set `self.DeltaTime` DeltaSeconds)
  (`|ExecutionSequence`
    (:`then_0`
      (`|ExecutionSequence`
        (:`then_0`
          (`|ExecutionSequence`
            (:`then_0`
              (set `self.CurrentFwdVector` (`KismetMathLibrary.VInterpTo` (`self.CurrentFwdVector`) (`self.TargetFwdVector`) (`self.DeltaTime`) (`self.GetMovementInterpSpeed`))))
            (:`then_1`
              (set `self.CurrentRightVector` (`KismetMathLibrary.VInterpTo` (`self.CurrentRightVector`) (`self.TargetRightVector`) (`self.DeltaTime`) (`self.GetMovementInterpSpeed`))))
            (:`then_2`
              (set `self.CurrentUpVector` (`KismetMathLibrary.VInterpTo` (`self.CurrentUpVector`) (`self.TargetUpVector`) (`self.DeltaTime`) (`self.GetMovementInterpSpeed`))))))
        (:`then_1`
          (`PawnMovementComponent.AddInputVector` (`self.FloatingPawnMovement`) (`self.ClampUpMovement` (`self.CurrentMovement`)) false))))
    (:`then_1`
      (switch `/Game/Gameplay/BeeAndBear/RotationMode` (`self.RotationMode`)
        (:`NewEnumerator1`
          (if (and (> (`KismetMathLibrary.VSize` (`self.GetVelocity`)) 0.0) (!= (`KismetMathLibrary.VSize` (`self.TargetMovement`)) 0.0))
            (`self.K2_SetActorRotation` (`KismetMathLibrary.RInterpTo` (`self.K2_GetActorRotation`) (`KismetMathLibrary.MakeRotator` 0.0 0.0 _returnvalue_yaw) (`self.DeltaTime`) 5.0))))))
    (:`then_2`
      (`self.UpdateRotationMode` (select `bool` (== (`KismetMathLibrary.VSize` (`self.TargetMovement`)) 0.0) :`false` "NewEnumerator0" :`true` "NewEnumerator1" :!type "/Game/Gameplay/BeeAndBear/RotationMode Enum")))
    (:`then_3`
      (`KismetSystemLibrary.PrintString` (`KismetStringLibrary.Concat_StrStr` "Honey Cubes Count: " (`KismetStringLibrary.Conv_IntToString` (`self.HoneyCubeCount`))) true true (struct :`G` 0.66 :`B` 1.0 :`A` 1.0) 0.0))))

(event `SnapCharToCamera`
  (params (InitialRotation :type "Rotator Structure"))
  (bind (_direction _value) (`Timeline|CharTimeline` :!via `PlayFromStart`)
    (:`Update`
      (`self.K2_SetActorRotation` (`KismetMathLibrary.RLerp` InitialRotation (`self.GetControlRotation`) _value true)))
    (:`Finished`
      (set `self.bUseControllerRotationYaw` true))))

(event `InputAxis|MoveFB`
  (params (AxisValue :type "Float (single-precision)"))
  (bind (_returnvalue_roll _returnvalue_pitch _returnvalue_yaw) (`KismetMathLibrary.BreakRotator` (`self.GetControlRotation`)))
  (bind _output_get (set `self.InputFB` AxisValue))
  (set `self.TargetRightVector` (* (`KismetMathLibrary.GetForwardVector` (`KismetMathLibrary.MakeRotator` 0.0 _returnvalue_pitch _returnvalue_yaw)) _output_get)))

(event `Key|One`
  (params (Key :type "Key Structure"))
  (:`Pressed`
    (switch `/Game/Gameplay/BeeAndBear/CameraMode` (`self.CurrentViewMode`)
      (:`NewEnumerator0`
        _)
      (:`NewEnumerator3`
        _))
    (`self.UpdateRotationMode` "NewEnumerator0")))

(event `InputAxis|MoveRL`
  (params (AxisValue :type "Float (single-precision)"))
  (bind (_returnvalue_roll _returnvalue_pitch _returnvalue_yaw) (`KismetMathLibrary.BreakRotator` (`self.GetControlRotation`)))
  (bind _output_get (set `self.InputRL` AxisValue))
  (set `self.TargetFwdVector` (* (`KismetMathLibrary.GetRightVector` (`KismetMathLibrary.MakeRotator` 0.0 _returnvalue_pitch _returnvalue_yaw)) _output_get)))

(event `Key|Two`
  (params (Key :type "Key Structure"))
  (:`Pressed`
    (switch `/Game/Gameplay/BeeAndBear/CameraMode` (`self.CurrentViewMode`)
      (:`NewEnumerator0`
        (`self.UpdateRotationMode` "NewEnumerator1")))))

(event `InputAxis|LookRL`
  (params (AxisValue :type "Float (single-precision)"))
  (`self.AddControllerYawInput` AxisValue))

(event `InputAxis|LookUD`
  (params (AxisValue :type "Float (single-precision)"))
  (`self.AddControllerPitchInput` AxisValue))

(event `InputAxis|MoveUD`
  (params (AxisValue :type "Float (single-precision)"))
  (set `self.TargetUpVector` (* (`self.GetActorUpVector`) AxisValue)))

(fn `ClampUpMovement`
  (params (in :type "Vector Structure"))
  (returns (out :type "Vector Structure"))
  (bind (_returnvalue_x _returnvalue_y _returnvalue_z) (`KismetMathLibrary.BreakVector` (`self.K2_GetActorLocation`)))
  (bind (_returnvalue_x_2 _returnvalue_y_2 _returnvalue_z_2) (`KismetMathLibrary.BreakVector` (`self.K2_GetActorLocation`)))
  (bind (_returnvalue_x_3 _returnvalue_y_3 _returnvalue_z_3) (`KismetMathLibrary.BreakVector` (`self.K2_GetActorLocation`)))
  (bind (_returnvalue_x_4 _returnvalue_y_4 _returnvalue_z_4) (`KismetMathLibrary.BreakVector` (`self.K2_GetActorLocation`)))
  (bind _maxheight (`self.MaxHeight`))
  (bind _maxheight_2 (`self.MaxHeight`))
  (bind (_in_x _in_y _in_z) (`KismetMathLibrary.BreakVector` (`local.in`)))
  (bind (_in_x_2 _in_y_2 _in_z_2) (`KismetMathLibrary.BreakVector` (`local.in`)))
  (bind (_in_x_3 _in_y_3 _in_z_3) (`KismetMathLibrary.BreakVector` (`local.in`)))
  (bind (_in_x_4 _in_y_4 _in_z_4) (`KismetMathLibrary.BreakVector` (`local.in`)))
  (bind _returnvalue (/ (`self.MaxHeight`) 2.0))
  (return (`KismetMathLibrary.MakeVector` (`KismetMathLibrary.MapRangeClamped` _returnvalue_z_4 (/ _maxheight_2 2.0) _maxheight_2 in_X (`KismetMathLibrary.MapRangeClamped` _in_z 0.0 1.0 in_X (/ in_X 3.0))) (`KismetMathLibrary.MapRangeClamped` _returnvalue_z_3 (/ _maxheight 2.0) _maxheight in_Y (`KismetMathLibrary.MapRangeClamped` _in_z 0.0 1.0 in_Y (/ in_Y 3.0))) (`KismetMathLibrary.SelectFloat` (`KismetMathLibrary.SelectFloat` _in_z_4 (`KismetMathLibrary.MapRangeClamped` _returnvalue_z_2 _returnvalue (`self.MaxHeight`) _in_z_2) (< _in_z_3 0.0)) in_Z (> _returnvalue_z _returnvalue)))))

(fn `GetCharacterMovementInfo`
  (returns (MovementInput :type "Vector Structure"))
  (return (`KismetMathLibrary.MakeVector` (`self.InputFB`) (`self.InputRL`))))

(fn `GetDesiredMovementAngle`
  (returns (OutAbgle :type "Float (double-precision)"))
  (return (`/Game/Gameplay/HH_FunctionsLib.GetAngleBetweenVectors` (`self.CurrentMovement`) (`self.TargetMovement`))))

(fn `RequestRemainingTime`
  (returns (OutTime :type "Float (double-precision)"))
  (return 0.0))

(fn `ToggleView`
  (if (>= (+ (`KismetMathLibrary.Conv_ByteToInt` (`self.CurrentViewMode`)) 1) (enumcount `/Game/Gameplay/BeeAndBear/CameraMode`))
    (`self.UpdateVIewMode` "NewEnumerator0")
    (else
      (`self.UpdateVIewMode` (cast `/Game/Gameplay/BeeAndBear/CameraMode` (`KismetMathLibrary.Conv_IntToByte` (+ (`KismetMathLibrary.Conv_ByteToInt` (`self.CurrentViewMode`)) 1)))))))

(fn `UpdateRotationMode`
  (params (RotationMode :type "/Game/Gameplay/BeeAndBear/RotationMode Enum" :default "NewEnumerator0"))
  (bind _output_get (set `self.RotationMode` RotationMode))
  (switch `/Game/Gameplay/BeeAndBear/RotationMode` (`self.RotationMode`)
    (:`NewEnumerator0`
      (`self.SnapCharToCamera` (`self.K2_GetActorRotation`)))
    (:`NewEnumerator1`
      (switch `/Game/Gameplay/BeeAndBear/CameraMode` (`self.CurrentViewMode`)
        (:`NewEnumerator0`
          (set `self.bUseControllerRotationYaw` false)
          (`|ExecutionSequence`
            (:`then_0`
              (set `SpringArmComponent.bUsePawnControlRotation` true (`self.SA_TP`))
              (set `SpringArmComponent.bInheritYaw` true (`self.SA_TP`))
              (set `SpringArmComponent.bInheritPitch` true (`self.SA_TP`)))))
        (:`NewEnumerator3`
          (set `self.bUseControllerRotationYaw` false))))))

(fn `UpdateVIewMode`
  (params (NewMode :type "/Game/Gameplay/BeeAndBear/CameraMode Enum" :default "NewEnumerator0"))
  (bind _output_get (set `self.CurrentViewMode` NewMode))
  (switch `/Game/Gameplay/BeeAndBear/CameraMode` _output_get
    (:`NewEnumerator0`
      (`ActorComponent.SetActive` (`self.Camera_TP`) true false)
      (`self.UpdateRotationMode` "NewEnumerator1"))
    (:`NewEnumerator1`
      (`ActorComponent.SetActive` (`self.Camera_TP`) false false)
      (`self.UpdateRotationMode` "NewEnumerator0"))
    (:`NewEnumerator3`
      (`ActorComponent.SetActive` (`self.Camera_TP`) false false)
      (`self.UpdateRotationMode` "NewEnumerator1"))))

(fn `UserConstructionScript`
  (`SceneComponent.SetAbsolute` (`self.Bear_01`) false false true)
  (`SceneComponent.SetWorldScale3D` (`self.Bear_01`) (`self.GetActorScale3D`))
  (`self.UpdateFromManagementTable`)
  (`TimelineComponent.SetPlayRate` (`self.CharTimeline`) 8.0))